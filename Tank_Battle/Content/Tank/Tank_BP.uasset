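; Player-controllable tank Blueprint with an orbiting aim camera and a fire action.
; On BeginPlay it registers its barrel and turret components through setter functions defined outside these graphs.
; Camera axes rotate the azimuth gimbal in yaw and the spring arm in pitch separately, scaled by frame delta time.
; The Fire input calls a Fire function whose logic also lives outside these graphs.
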(event EventBeginPlay
  (Class|Tank|SetBarrelReference (Variables|Default|GetTankBarrel))
  (Class|Tank|SetTurretReference (Variables|Default|GetTankTurret)))

(event Input|ActionEvents|InputActionFire
  (params (Key :type Key%20Structure))
  (:Pressed
    (Class|Tank|Fire)))

(event Input|AxisEvents|InputAxisCameraAzimuth
  (params (AxisValue :type Float%20%28single-precision%29))
  (Transformation|AddLocalRotation (Variables|Default|GetAzimat%20Gimbal) (Math|Rotator|MakeRotator 0.0 0.0 (* AxisValue (Utilities|Time|GetWorldDeltaSeconds) 1e+02)) false false))

(event Input|AxisEvents|InputAxisCameraElavation
  (params (AxisValue :type Float%20%28single-precision%29))
  (Transformation|AddLocalRotation (Variables|Default|GetSpringArm) (Math|Rotator|MakeRotator 0.0 (* AxisValue (Utilities|Time|GetWorldDeltaSeconds) 1e+02) 0.0) false false))

(fn ConstructionScript)